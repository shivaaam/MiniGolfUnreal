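; Mini-golf hole actor that completes the current level through the GolfGameMode's scene info when the player pawn overlaps it.
; On BeginPlay it reads the magnetic-hole skill radius from GolfGameInstance, flags the magnet active if positive, and scales the MagneticField component to that radius.
; Tick syncs the field's visibility to that flag; no attraction force is applied in this graph.
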(event `self.ReceiveBeginPlay`
  (bind _magnetradius (`self.magnetRadius`))
  (bind _asgolf_game_instance (cast `/Game/_MiniGolf/Blueprints/Managers/GolfGameInstance` (`GameplayStatics.GetGameInstance`)))
  (bind _skill_magneticholeradius (`/Game/_MiniGolf/Blueprints/Managers/GolfGameInstance.skill_magneticHoleRadius` _asgolf_game_instance))
  (`KismetSystemLibrary.PrintString` (`KismetStringLibrary.Conv_DoubleToString` _skill_magneticholeradius) true true (struct :`R` 0.977146 :`G` 1.0 :`B` 0.914102 :`A` 1.0) 5.0)
  (set `self.magnetRadius` _skill_magneticholeradius)
  (set `self.isMagnetActive` (> _magnetradius 0.0))
  (`SceneComponent.SetRelativeScale3D` (`self.magneticField`) (`KismetMathLibrary.MakeVector` _magnetradius _magnetradius _magnetradius)))

(event `self.ReceiveActorBeginOverlap`
  (params (OtherActor :type "Actor Object Reference"))
  (`self.CheckForPAR` OtherActor))

(event `self.ReceiveActorEndOverlap`
  (params (OtherActor :type "Actor Object Reference"))
  (if (== OtherActor (`GameplayStatics.GetPlayerController` 0))
    (`KismetSystemLibrary.PrintString` "OnTriggerExit")))

(event `self.ReceiveTick`
  (params (DeltaSeconds :type "Float (single-precision)"))
  (`SceneComponent.SetVisibility` (`self.magneticField`) (`self.isMagnetActive`) false))

(fn `CheckForPAR`
  (params (other :type "Actor Object Reference"))
  (if (== other (`GameplayStatics.GetPlayerPawn` 0))
    (`KismetSystemLibrary.PrintString` (`KismetSystemLibrary.GetDisplayName` other))
    (bind _asgolf_game_mode (cast `/Game/_MiniGolf/Blueprints/Managers/GolfGameMode` (`GameplayStatics.GetGameMode`)))
    (`/Game/_MiniGolf/Blueprints/Managers/SceneInfo.CompleteCurrentLevel` (`/Game/_MiniGolf/Blueprints/Managers/GolfGameMode.currentSceneInfo` _asgolf_game_mode))))

(fn `UserConstructionScript`)