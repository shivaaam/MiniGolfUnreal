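; Mini-golf game instance that holds persistent player progress: collected coins, three skill levels and their current values, and cleared levels.
; Init seeds launch power, laser sight distance and magnetic hole radius from the first entry of each SkillUpgrades array.
; BuyUpgrade routes an ID to a per-skill purchase that checks the next level's cost, deducts coins, raises the level and caches the new value.
; Helpers reset coins and record cleared levels.
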(event `self.ReceiveInit`
  (bind _output (`self.GetSkill0UpgradeAtIndex` 0))
  (set `self.skill_maxLaunchPower` (`.value_3_8B28506D4D4A274F916784A9501C7437` (break `/Game/_MiniGolf/Blueprints/Managers/Struct_SkillLevelData` _output)))
  (bind _output_2 (`self.GetSkill1UpgradeAtIndex` 0))
  (set `self.skill_laserSightDistance` (`.value_3_8B28506D4D4A274F916784A9501C7437` (break `/Game/_MiniGolf/Blueprints/Managers/Struct_SkillLevelData` _output_2)))
  (bind _output_3 (`self.GetSkill2UpgradeAtIndex` 0))
  (set `self.skill_magneticHoleRadius` (`.value_3_8B28506D4D4A274F916784A9501C7437` (break `/Game/_MiniGolf/Blueprints/Managers/Struct_SkillLevelData` _output_3))))

(fn `AddToClearedLevels`
  (params (levelId :type String))
  (bind _output_get (set `self.levelsCleared` (`self.levelsCleared`)))
  (bind _returnvalue (`KismetArrayLibrary.Array_Add` _output_get levelId))
  (`KismetSystemLibrary.PrintString` (`KismetStringLibrary.Conv_IntToString` _returnvalue) true true (struct :`R` 1.0 :`G` 0.329681 :`B` 0.967051 :`A` 1.0)))

(fn `BuyUpgrade`
  (params (upgradeId :type Integer))
  (switch `int` upgradeId
    (:`0`
      (`self.BuyUpgrade_LaunchPower`))
    (:`1`
      (`self.BuyUpgrade_LaserSight`))
    (:`2`
      (`self.BuyUpgrade_MagneticHole`))))

(fn `BuyUpgrade_LaserSight`
  (bind _returnvalue (+ (`self.skillLevel_1`) 1))
  (bind _output (`self.GetSkill1UpgradeAtIndex` _returnvalue))
  (bind (_value _cost) (break `/Game/_MiniGolf/Blueprints/Managers/Struct_SkillLevelData` _output))
  (if (>= (`self.coinsCollected`) _cost)
    (`self.DeductCoins` _cost)
    (bind _output_get (set `self.skillLevel_1` _returnvalue))
    (bind _output_2 (`self.GetSkill1UpgradeAtIndex` _output_get))
    (`KismetSystemLibrary.PrintString` (`KismetStringLibrary.Concat_StrStr` "laser sight level: " (`KismetStringLibrary.Conv_IntToString` _output_get)))
    (set `self.skill_laserSightDistance` (`.value_3_8B28506D4D4A274F916784A9501C7437` (break `/Game/_MiniGolf/Blueprints/Managers/Struct_SkillLevelData` _output_2)))))

(fn `BuyUpgrade_LaunchPower`
  (bind _returnvalue (+ (`self.skillLevel_0`) 1))
  (bind _output (`self.GetSkill0UpgradeAtIndex` _returnvalue))
  (bind (_value _cost) (break `/Game/_MiniGolf/Blueprints/Managers/Struct_SkillLevelData` _output))
  (if (>= (`self.coinsCollected`) _cost)
    (`self.DeductCoins` _cost)
    (bind _output_get (set `self.skillLevel_0` _returnvalue))
    (bind _output_2 (`self.GetSkill0UpgradeAtIndex` _output_get))
    (bind _value_2 (break `/Game/_MiniGolf/Blueprints/Managers/Struct_SkillLevelData` _output_2))
    (`KismetSystemLibrary.PrintString` (`KismetStringLibrary.Concat_StrStr` (`KismetStringLibrary.Concat_StrStr` (`KismetStringLibrary.Concat_StrStr` "launch power level: " (`KismetStringLibrary.Conv_IntToString` _output_get)) " | ") (`KismetStringLibrary.Conv_DoubleToString` _value_2)))
    (set `self.skill_maxLaunchPower` _value_2)))

(fn `BuyUpgrade_MagneticHole`
  (bind _returnvalue (+ (`self.skillLevel_2`) 1))
  (bind _output (`self.GetSkill2UpgradeAtIndex` _returnvalue))
  (bind (_value _cost) (break `/Game/_MiniGolf/Blueprints/Managers/Struct_SkillLevelData` _output))
  (if (>= (`self.coinsCollected`) _cost)
    (`self.DeductCoins` _cost)
    (bind _output_get (set `self.skillLevel_2` _returnvalue))
    (bind _output_2 (`self.GetSkill2UpgradeAtIndex` _output_get))
    (`KismetSystemLibrary.PrintString` (`KismetStringLibrary.Concat_StrStr` "magnetic hole level: " (`KismetStringLibrary.Conv_IntToString` _output_get)))
    (set `self.skill_magneticHoleRadius` (`.value_3_8B28506D4D4A274F916784A9501C7437` (break `/Game/_MiniGolf/Blueprints/Managers/Struct_SkillLevelData` _output_2)))))

(fn `DeductCoins`
  (params (amount :type Integer))
  (set `self.coinsCollected` (- (`self.coinsCollected`) amount)))

(fn `GetSkill0UpgradeAtIndex`
  (params (index :type Integer))
  (returns (Output :type "/Game/_MiniGolf/Blueprints/Managers/Struct_SkillLevelData Structure"))
  (return (`|GetArrayItem` (`.launchPower_7_9F4B3DB24AC7DCDE274C82B8F3163AA2` (break `/Game/_MiniGolf/Blueprints/Managers/Struct_Skills` (`self.skillUpgrades`))) index)))

(fn `GetSkill1UpgradeAtIndex`
  (params (index :type Integer))
  (returns (Output :type "/Game/_MiniGolf/Blueprints/Managers/Struct_SkillLevelData Structure"))
  (return (`|GetArrayItem` (`.laserSight_8_377096F24CFBFB188785E4A40483EFE0` (break `/Game/_MiniGolf/Blueprints/Managers/Struct_Skills` (`self.skillUpgrades`))) index)))

(fn `GetSkill2UpgradeAtIndex`
  (params (index :type Integer))
  (returns (Output :type "/Game/_MiniGolf/Blueprints/Managers/Struct_SkillLevelData Structure"))
  (return (`|GetArrayItem` (`.magneticHole_9_1760E5944FA5053523DEE0A2F6BAAC4A` (break `/Game/_MiniGolf/Blueprints/Managers/Struct_Skills` (`self.skillUpgrades`))) index)))

(fn `ResetCoins`
  (set `self.coinsCollected` 0))