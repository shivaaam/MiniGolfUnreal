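; Player-controlled minigolf ball that handles aiming, charged shots and settling to rest, with color and max power read from GolfGameInstance.
; Mouse movement drives camera and shot yaw, the wheel sets pitch, and a debug arrow previews launch direction.
; While stationary, holding left mouse charges power and releasing sets the CCD-enabled physics mesh's velocity.
; Tick checks speed, applying manual counter-force friction when slow and zeroing velocity below the movement threshold.
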(event `self.ReceiveBeginPlay`
  ;[0.08618 0.631 1] Enable CCD (Continuous collision detection)
  (`PrimitiveComponent.SetUseCCD` (`self.GolfBallMesh`) true "None")
  ;[1 0.6916 0.1896] Set ball color
  (bind _asgolf_game_instance (cast `/Game/_MiniGolf/Blueprints/Managers/GolfGameInstance` (`GameplayStatics.GetGameInstance`)))
  (bind _ballcolor (`/Game/_MiniGolf/Blueprints/Managers/GolfGameInstance.ballColor` _asgolf_game_instance))
  (`KismetSystemLibrary.PrintString` (`KismetStringLibrary.Conv_ColorToString` _ballcolor))
  (`self.SetBallColor` _ballcolor))

(event `InputAxisKey|MouseX`
  (params (AxisValue :type "Float (single-precision)"))
  ;[1 1 1] Camera Handling
  (`self.AddControllerYawInput` AxisValue)
  ;[1 1 1] Set shot launch direction
  (`self.SetShotYaw`)
  (`self.SetLaunchDirection` :!label _label))

(event `self.ReceiveTick`
  (params (DeltaSeconds :type "Float (single-precision)"))
  (set `self.deltaTime` DeltaSeconds)
  (`self.DrawShotDirectionArrow`)
  (`self.SetIsMoving`)
  (`KismetSystemLibrary.PrintString` (`KismetStringLibrary.Conv_BoolToString` (`self.isMoving`)) true true (struct :`R` 1.0 :`G` 0.009009 :`A` 1.0) 0.0)
  (`KismetSystemLibrary.PrintString` (`KismetStringLibrary.Conv_DoubleToString` (`self.currentShotPower`)) true true (struct :`G` 0.897796 :`B` 1.0 :`A` 1.0) 0.0)
  (if (and (`self.isCharging`) (not (`self.isMoving`)))
    (`self.IncreaseLaunchPower`)))

(event `InputAxisKey|MouseY`
  (params (AxisValue :type "Float (single-precision)"))
  ;[1 1 1] Camera Handling
  (`self.SetMinMaxCameraPitch` 290.0 345.0)
  (`self.AddControllerPitchInput` (* -1 AxisValue)))

(event `InputAxisKey|MouseWheelAxis`
  (params (AxisValue :type "Float (single-precision)"))
  ;[1 1 1] Set shot launch direction
  (`self.SetShotPitch` AxisValue)
  (goto _label))

(event `Key|LeftMouseButton`
  (params (Key :type "Key Structure"))
  (bind _ismoving (`self.isMoving`))
  ;[1 1 1] Take Shot
  (:`Pressed`
    (if (not _ismoving)
      (set `self.isCharging` true)))
  (:`Released`
    (if (not _ismoving)
      (`self.TakeShot`)
      (`self.OnTakeShot`))))

(fn `ApplyManualFriction`
  (bind _golfballmesh (`self.GolfBallMesh`))
  (if (<= (`self.currentVelocity`) (`self.applyFrictionThreshold`))
    (`PrimitiveComponent.AddForce` _golfballmesh (* (* (`SceneComponent.GetComponentVelocity` _golfballmesh) -1.0) 0.65) "None" false)))

(fn `DrawShotDirectionArrow`
  (bind _returnvalue (`self.K2_GetActorLocation`))
  (if (not (`self.isMoving`))
    (`KismetSystemLibrary.DrawDebugArrow` _returnvalue (+ _returnvalue (* (`self.launchDirection`) (`self.arrowLength`))) 10.0 (struct :`R` 0.181332 :`G` 1.0 :`B` 0.056041 :`A` 1.0) 0.0 1.0)))

(fn `IncreaseLaunchPower`
  (bind _returnvalue (+ (`self.currentShotPower`) (* (`self.deltaTime`) (`self.launchPowerIncrementRate`))))
  (`self.SetLaunchPower` _returnvalue)
  (`KismetSystemLibrary.PrintString` (`KismetStringLibrary.Conv_DoubleToString` _returnvalue) true true (struct :`G` 0.66 :`B` 1.0 :`A` 1.0) 0.0))

(fn `OnTakeShot`
  (set `self.isCharging` false)
  (`self.ResetLaunchPower`)
  (`self.ResetLaunchDirection`))

(fn `ResetLaunchDirection`
  (set `self.currentShotPitch` 0.0))

(fn `ResetLaunchPower`
  (set `self.currentShotPower` 0.0))

(fn `SetBallColor`
  (params (color :type "LinearColor Structure"))
  (bind _returnvalue (`PrimitiveComponent.CreateDynamicMaterialInstance` (`self.GolfBallMesh`) 0 null "None"))
  (`MaterialInstanceDynamic.SetVectorParameterValue` _returnvalue "None" color)
  (`PrimitiveComponent.SetMaterial` (`self.GolfBallMesh`) 0 null))

(fn `SetIsMoving`
  (bind _output_get (set `self.currentVelocity` (`KismetMathLibrary.VSize` (`SceneComponent.GetComponentVelocity` (`self.GolfBallMesh`)))))
  (`KismetSystemLibrary.PrintString` (`KismetStringLibrary.Conv_DoubleToString` _output_get) true true (struct :`R` 1.0 :`G` 0.946138 :`A` 1.0) 0.0)
  (bind _output_get_2 (set `self.isMoving` (> _output_get (`self.isMovingThreshold`))))
  (if _output_get_2
    (`self.ApplyManualFriction`)
    (else
      (`self.StopAllMovement`))))

(fn `SetLaunchDirection`
  (set `self.launchDirection` (`KismetMathLibrary.GetForwardVector` (`KismetMathLibrary.MakeRotator` 0.0 (`self.currentShotPitch`) (`self.currentShotYaw`)))))

(fn `SetLaunchPower`
  (params (power :type "Float (double-precision)"))
  (bind _asgolf_game_instance (cast `/Game/_MiniGolf/Blueprints/Managers/GolfGameInstance` (`GameplayStatics.GetGameInstance`)))
  (set `self.currentShotPower` (`KismetMathLibrary.FClamp` power 0.0 (`/Game/_MiniGolf/Blueprints/Managers/GolfGameInstance.maxLaunchPower` _asgolf_game_instance))))

(fn `SetMinMaxCameraPitch`
  (params (min :type "Float (double-precision)") (max :type "Float (double-precision)"))
  (bind _returnvalue (`GameplayStatics.GetPlayerCameraManager` 0))
  (set `PlayerCameraManager.ViewPitchMin` min _returnvalue)
  (set `PlayerCameraManager.ViewPitchMax` max _returnvalue))

(fn `SetShotPitch`
  (params (mouseScrollVal :type "Float (double-precision)"))
  (bind _returnvalue (`KismetMathLibrary.FClamp` (+ (`self.currentShotPitch`) (* mouseScrollVal (`self.anglesPerScroll`))) -45.0 80.0))
  (`KismetSystemLibrary.PrintString` (`KismetStringLibrary.Conv_DoubleToString` _returnvalue) true true (struct :`R` 0.07485 :`G` 1.0 :`B` 0.164862 :`A` 1.0) 0.0)
  (set `self.currentShotPitch` _returnvalue))

(fn `SetShotYaw`
  (set `self.currentShotYaw` (.yaw (`self.GetControlRotation`))))

(fn `StopAllMovement`
  (`PrimitiveComponent.SetPhysicsLinearVelocity` (`self.GolfBallMesh`) (0.0 0.0 0.0) false "None"))

(fn `TakeShot`
  (`PrimitiveComponent.SetPhysicsLinearVelocity` (`self.GolfBallMesh`) (* (`self.launchDirection`) (`self.currentShotPower`)) false "None"))

(fn `UserConstructionScript`)