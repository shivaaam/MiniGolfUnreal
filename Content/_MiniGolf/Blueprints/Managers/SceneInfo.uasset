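; Per-level manager actor for the mini golf game that spawns the player's ball and handles level completion.
; On BeginPlay it registers itself with GolfGameMode, finds the Hole if unset, then spawns and possesses a GolfBall at the PlayerStart.
; Tick updates the truncated ball-to-hole distance.
; CompleteCurrentLevel fires a dispatcher that shows the completion widget with UI-only input, and LoadNextLevel opens the referenced next level.
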(event `self.ReceiveBeginPlay`
  ;[1 0.6443 0] Bind Events
  (add `self.OnLevelComeplete` (delegate `LevelEnd`))
  (`self.UpdateReferenceInGameMode`)
  ;[1 1 1] Set 'ballHole' reference if it is not set
  (`self.SetLevelPAR`)
  ;[1 1 1] Spawn Player on level loaded
  (bind _spawnedaactor (`self.SpawnPlayer`))
  (`self.SetPlayerPawn` _spawnedaactor)
  (`WidgetBlueprintLibrary.SetInputMode_GameOnly` (`GameplayStatics.GetPlayerController` 0)))

(event `self.ReceiveTick`
  (params (DeltaSeconds :type "Float (single-precision)"))
  (`self.Set Par Distance`))

(event `LevelEnd`
  (params (levelName :type String))
  (`KismetSystemLibrary.PrintString` (`KismetStringLibrary.Concat_StrStr` "level end: " levelName))
  (`self.Show Level Completion Widget`))

(fn `CompleteCurrentLevel`
  (`self.OnLevelComeplete` (`self.levelName`)))

(fn `LevelCompletionDelegate`
  (params (levelName :type String)))

(fn `LoadNextLevel`
  (`GameplayStatics.OpenLevelBySoftObjectPtr` (`self.nextLevel`)))

(fn `Set Par Distance`
  (bind _truncatedval (`self.TruncateToNDecimals` (/ (`KismetMathLibrary.Vector_Distance` (`self.K2_GetActorLocation` (`self.playerPawn`)) (`self.K2_GetActorLocation` (`self.ballHole`))) 100.0)))
  (set `self.distanceToHole` _truncatedval))

(fn `SetLevelCompletionWidgetDetails`)

(fn `SetLevelPAR`
  (`/Engine/EditorBlueprintResources/StandardMacros.IsValid` (`self.ballHole`)
    (:`Is Not Valid`
      (bind _returnvalue (`GameplayStatics.GetActorOfClass` "/Game/_MiniGolf/Blueprints/GameComponents/Hole.Hole_C"))
      (set `self.ballHole` _returnvalue))))

(fn `SetPlayerPawn`
  (params (pawnActor :type "/Game/_MiniGolf/Blueprints/GameComponents/GolfBall Object Reference"))
  (set `self.playerPawn` pawnActor))

(fn `Show Level Completion Widget`
  (bind _returnvalue (`|CreateWidget` "/Game/_MiniGolf/Widgets/Widget_4LevelComplete.Widget_4LevelComplete_C"))
  (`UserWidget.AddToViewport` _returnvalue 0)
  (`WidgetBlueprintLibrary.SetInputMode_UIOnlyEx` (`GameplayStatics.GetPlayerController` 0) _returnvalue))

(fn `SpawnPlayer`
  (returns (spawnedAactor :type "/Game/_MiniGolf/Blueprints/GameComponents/GolfBall Object Reference"))
  (bind _returnvalue (`GameplayStatics.GetActorOfClass` "/Script/Engine.PlayerStart"))
  (bind _returnvalue_2 (`|SpawnActorFromClass` "/Game/_MiniGolf/Blueprints/GameComponents/GolfBall.GolfBall_C" (`KismetMathLibrary.MakeTransform` (.location (`self.GetTransform` _returnvalue)) (.rotation (`self.GetTransform` _returnvalue))) "AlwaysSpawn" "OverrideRootScale" null null))
  (`KismetSystemLibrary.PrintString` (`KismetStringLibrary.Concat_StrStr` "player spawned: " (`KismetSystemLibrary.GetDisplayName` _returnvalue_2)))
  (`self.SetActorScale3D` _returnvalue_2 (1.0 1.0 1.0))
  (`Controller.Possess` (`GameplayStatics.GetPlayerController` 0) _returnvalue_2)
  (return _returnvalue_2))

(fn `TruncateToNDecimals`
  (params (val :type "Float (double-precision)"))
  (returns (truncatedVal :type "Float (double-precision)"))
  (bind _truncatefactor (`self.truncateFactor`))
  (return (/ (`KismetMathLibrary.Conv_IntToDouble` (`KismetMathLibrary.FFloor` (* val _truncatefactor))) _truncatefactor)))

(fn `UpdateReferenceInGameMode`
  (bind _asgolf_game_mode (cast `/Game/_MiniGolf/Blueprints/Managers/GolfGameMode` (`GameplayStatics.GetGameMode`)))
  (set `/Game/_MiniGolf/Blueprints/Managers/GolfGameMode.currentSceneInfo` self _asgolf_game_mode))

(fn `UserConstructionScript`)