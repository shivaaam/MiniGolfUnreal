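; CoinBP is a collectible coin for the mini golf game that is collected and destroyed when any actor overlaps it.
; Overlap increments the coin count in GolfGameInstance and in the GolfGameMode's current scene info, then plays a pickup sound at world origin.
; The construction script also increments the GameInstance count.
; The spark particle spawn is left disconnected, so that step does nothing.
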(event `self.ReceiveActorBeginOverlap`
  (params (OtherActor :type "Actor Object Reference"))
  (`self.IncreaseCollectedCoins`)
  (`self.SpawnCoinCollectParticles`)
  (`self.PlayCollectSound`)
  (`self.K2_DestroyActor`))

(fn `IncreaseCollectedCoins`
  ;[1 1 1] Game Instance
  (bind _asgolf_game_instance (cast `/Game/_MiniGolf/Blueprints/Managers/GolfGameInstance` (`GameplayStatics.GetGameInstance`)))
  (set `/Game/_MiniGolf/Blueprints/Managers/GolfGameInstance.coinsCollected` (+ (`/Game/_MiniGolf/Blueprints/Managers/GolfGameInstance.coinsCollected` _asgolf_game_instance) 1) _asgolf_game_instance)
  ;[1 1 1] Scene Info
  (bind _asgolf_game_mode (cast `/Game/_MiniGolf/Blueprints/Managers/GolfGameMode` (`GameplayStatics.GetGameMode`)))
  (bind _currentsceneinfo (`/Game/_MiniGolf/Blueprints/Managers/GolfGameMode.currentSceneInfo` _asgolf_game_mode))
  (set `/Game/_MiniGolf/Blueprints/Managers/SceneInfo.coinsCollected` (+ (`/Game/_MiniGolf/Blueprints/Managers/SceneInfo.coinsCollected` _currentsceneinfo) 1) _currentsceneinfo))

(fn `PlayCollectSound`
  (`GameplayStatics.PlaySoundAtLocation` "/Game/_MiniGolf/Sounds/SFXs/pickup.pickup" (0.0 0.0 0.0) (struct) 1.0 1.0 0.0 null null null))

(fn `SpawnCoinCollectParticles`)

(fn `UserConstructionScript`
  (bind _asgolf_game_instance (cast `/Game/_MiniGolf/Blueprints/Managers/GolfGameInstance` (`GameplayStatics.GetGameInstance`)))
  (set `/Game/_MiniGolf/Blueprints/Managers/GolfGameInstance.coinsCollected` (+ (`/Game/_MiniGolf/Blueprints/Managers/GolfGameInstance.coinsCollected` _asgolf_game_instance) 1) _asgolf_game_instance))