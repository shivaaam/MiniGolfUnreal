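; Player-controlled mini-golf ball that is aimed with the mouse, charged by holding left click and launched on release as a physics velocity.
; Game instance supplies ball color and skill limits for power and laser length.
; Tick updates the arrow, applies low-speed friction and steers the ball into the hole's magnet radius.
; At rest, a recursive line trace draws a bouncing laser sight with reused beam emitters, ignoring coins.
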(event `OnLevelComplete`
  (params (levelName :type String))
  (bind _golfballmesh (`self.GolfBallMesh`))
  ;[1 1 1] Turn off collision on level complete
  (`PrimitiveComponent.SetCollisionProfileName` _golfballmesh "NoCollision" true)
  (`PrimitiveComponent.SetSimulatePhysics` _golfballmesh false))

(event `self.ReceiveBeginPlay`
  ;[1 1 1] Bind to OnLevelComplete
  (bind _asgolf_game_mode (cast `/Game/_MiniGolf/Blueprints/Managers/GolfGameMode` (`GameplayStatics.GetGameMode`)))
  (add `/Game/_MiniGolf/Blueprints/Managers/SceneInfo.OnLevelComeplete` (`/Game/_MiniGolf/Blueprints/Managers/GolfGameMode.currentSceneInfo` _asgolf_game_mode) (delegate `OnLevelComplete`))
  ;[0.08618 0.631 1] Enable CCD (Continuous collision detection)
  (`PrimitiveComponent.SetUseCCD` (`self.GolfBallMesh`) true "None")
  ;[1 0.6916 0.1896] Set ball color
  (bind _asgolf_game_instance (cast `/Game/_MiniGolf/Blueprints/Managers/GolfGameInstance` (`GameplayStatics.GetGameInstance`)))
  (bind _ballcolor (`/Game/_MiniGolf/Blueprints/Managers/GolfGameInstance.ballColor` _asgolf_game_instance))
  (`KismetSystemLibrary.PrintString` (`KismetStringLibrary.Conv_ColorToString` _ballcolor) true true (struct :`R` 1.0 :`G` 0.04144 :`B` 0.061336 :`A` 1.0))
  (`self.SetBallColor` _ballcolor)
  ;[1 1 1] Set laser sight length
  (bind _asgolf_game_instance_2 (cast `/Game/_MiniGolf/Blueprints/Managers/GolfGameInstance` (`GameplayStatics.GetGameInstance`)))
  (bind _output_get (set `self.laserSightLength` (`/Game/_MiniGolf/Blueprints/Managers/GolfGameInstance.skill_laserSightDistance` _asgolf_game_instance_2)))
  (`KismetSystemLibrary.PrintString` (`KismetStringLibrary.Conv_DoubleToString` _output_get) true true (struct :`R` 0.933301 :`G` 1.0 :`B` 0.942927 :`A` 1.0) 5.0)
  (set `self.isLaserSightEnabled` (> _output_get 0.0)))

(event `InputAxisKey|MouseX`
  (params (AxisValue :type "Float (single-precision)"))
  ;[1 1 1] Camera Handling
  (`self.AddControllerYawInput` AxisValue)
  ;[1 1 1] Set shot launch direction
  (`self.SetShotYaw`)
  (`self.SetLaunchDirection` :!label _label))

(event `InputAxisKey|MouseWheelAxis`
  (params (AxisValue :type "Float (single-precision)"))
  ;[1 1 1] Set shot launch direction
  (if (not (`self.isMoving`))
    (bind _pitchangle (`self.SetShotPitch` AxisValue))
    (`self.UpdateShotPitchUI` _pitchangle)
    (goto _label)))

(event `InputAxisKey|MouseY`
  (params (AxisValue :type "Float (single-precision)"))
  ;[1 1 1] Camera Handling
  (`self.SetMinMaxCameraPitch` 290.0 345.0)
  (`self.AddControllerPitchInput` (* -1 AxisValue)))

(event `Key|LeftMouseButton`
  (params (Key :type "Key Structure"))
  (bind _returnvalue (not (`self.isMoving`)))
  ;[1 1 1] Take Shot
  (:`Pressed`
    (if _returnvalue
      (set `self.isCharging` true)))
  (:`Released`
    (if _returnvalue
      (`self.SetLastLaunchPosition` (`self.K2_GetActorLocation`))
      (`self.TakeShot`)
      (`self.OnTakeShot`))))

(event `self.ReceiveTick`
  (params (DeltaSeconds :type "Float (single-precision)"))
  (bind _lasersightparticles (`self.laserSightParticles`))
  (bind _returnvalue (`KismetArrayLibrary.Array_Length` _lasersightparticles))
  ;[1 1 1] Update Loop
  (set `self.deltaTime` DeltaSeconds)
  (`self.DrawShotDirectionArrow`)
  (`self.SetIsMoving`)
  (`self.SteerTowardsHole`)
  (`KismetSystemLibrary.PrintString` (`KismetStringLibrary.Conv_BoolToString` (`self.isMoving`)) true true (struct :`R` 1.0 :`G` 0.009009 :`A` 1.0) 0.0)
  (`KismetSystemLibrary.PrintString` (`KismetStringLibrary.Conv_DoubleToString` (`self.currentShotPower`)) true true (struct :`G` 0.897796 :`B` 1.0 :`A` 1.0) 0.0)
  (if (not (`self.isMoving`))
    (set `self.isLaserAllowed` true)
    (if (and (`self.isLaserSightEnabled`) (`self.isLaserAllowed`))
      (bind _outactors (`GameplayStatics.GetAllActorsOfClass` "/Game/_MiniGolf/Blueprints/GameComponents/CoinBP.CoinBP_C"))
      (set `self.raycastIgnoreActors` _outactors)
      (`self.DrawLaserSight` (`self.K2_GetActorLocation`) (`self.laserSightLength`) (`self.launchDirection`) (`self.raycastIgnoreActors`)))
    ;;[1 0.7707 0.1674] Set rays count
    (bind _output_get (set `self.currentLaserRays` (`self.currentLaserRaysTemp`)))
    (set `self.currentLaserRaysTemp` 0)
    (if (> _returnvalue _output_get)
      ;;[0.8073 0 0.01857] Remove extra laser particles
      (for _index (range _output_get _returnvalue)
        (bind _output (`|GetArrayItem` _lasersightparticles _index))
        (`ActorComponent.K2_DestroyComponent` _output)
        (`KismetArrayLibrary.Array_RemoveItem` _lasersightparticles _output)))
    (if (`self.isCharging`)
      (`self.IncreaseLaunchPower`)
      (bind _asgolf_game_instance (cast `/Game/_MiniGolf/Blueprints/Managers/GolfGameInstance` (`GameplayStatics.GetGameInstance`)))
      (`self.MultiplyArrowScale` (/ (`self.currentShotPower`) (`/Game/_MiniGolf/Blueprints/Managers/GolfGameInstance.skill_maxLaunchPower` _asgolf_game_instance))))))

(fn `ApplyManualFriction`
  (bind _golfballmesh (`self.GolfBallMesh`))
  (if (<= (`self.currentVelocity`) (`self.applyFrictionThreshold`))
    (`PrimitiveComponent.AddForce` _golfballmesh (* (* (`SceneComponent.GetComponentVelocity` _golfballmesh) -1.0) 0.65) "None" false)))

(fn `DrawLaserSight`
  (params (rayStartPosition :type "Vector Structure") (rayLength :type "Float (double-precision)") (rayDirection :type "Vector Structure") (ignoreActors :type "Array of Actor Object Reference"))
  (locals (remainingLength :type "Float (double-precision)") (rayDir :type "Vector Structure") (drawLength :type "Float (double-precision)") (rayStartPos :type "Vector Structure") (recursiveCallsCount :type Integer) (beamTargetLocation :type "Vector Structure") (laserParticle :type "ParticleSystemComponent Object Reference"))
  (bind _lasersightparticles (`self.laserSightParticles`))
  (bind _lasersightparticles_2 (`self.laserSightParticles`))
  (bind _currentlaserraystemp (`self.currentLaserRaysTemp`))
  (bind _laserparticle (`local.laserParticle`))
  (bind _laserparticle_2 (`local.laserParticle`))
  (bind _raystartpos (`local.rayStartPos`))
  (bind _returnvalue (- (`self.currentLaserRaysTemp`) 1))
  ;[1 1 1] Initialize variables
  (bind _output_get (set `local.remainingLength` rayLength))
  (set `local.rayDir` rayDirection)
  (set `local.drawLength` _output_get)
  (set `local.rayStartPos` rayStartPosition)
  (set `self.currentLaserRaysTemp` (+ (`self.currentLaserRaysTemp`) 1))
  (bind (_outhit _returnvalue_2) (`KismetSystemLibrary.LineTraceSingle` (`local.rayStartPos`) (+ (`local.rayStartPos`) (* (`KismetMathLibrary.Normal` (`local.rayDir`)) (`local.drawLength`))) "TraceTypeQuery1" true ignoreActors))
  (if _returnvalue_2
    (bind (_bblockinghit _binitialoverlap _time _distance _location _impactpoint _normal) (`GameplayStatics.BreakHitResult` _outhit))
    (set `local.beamTargetLocation` _impactpoint)
    (else
      (set `local.beamTargetLocation` (+ (`local.rayStartPos`) (* (`local.rayDir`) (`local.drawLength`))))))
  (if (<= _currentlaserraystemp (`KismetArrayLibrary.Array_Length` _lasersightparticles_2))
    (set `local.laserParticle` (`|GetArrayItem` _lasersightparticles_2 (- _currentlaserraystemp 1)))
    (else
      (bind _returnvalue_3 (`GameplayStatics.SpawnEmitterAtLocation` "/Game/_MiniGolf/Particles/Particle_LaserSight.Particle_LaserSight" _raystartpos))
      (set `local.laserParticle` _returnvalue_3)))
  (`ParticleSystemComponent.SetBeamSourcePoint` _laserparticle_2 0 _raystartpos 0)
  (`ParticleSystemComponent.SetBeamTargetPoint` _laserparticle_2 0 (`local.beamTargetLocation`) 0)
  (if (`KismetArrayLibrary.Array_IsValidIndex` _lasersightparticles _returnvalue)
    (`KismetArrayLibrary.Array_Set` _lasersightparticles _returnvalue _laserparticle)
    (else
      (`KismetArrayLibrary.Array_Insert` _lasersightparticles _laserparticle _returnvalue)))
  (if _returnvalue_2
    ;[1 1 1] Recursive Call
    (set `local.drawLength` _distance)
    (bind _output_get_2 (set `local.remainingLength` (- (`local.remainingLength`) _distance)))
    (bind _output_get_3 (set `local.rayDir` (`KismetMathLibrary.GetReflectionVector` (`local.rayDir`) _normal)))
    (bind _output_get_4 (set `local.rayStartPos` _impactpoint))
    (`self.DrawLaserSight` _output_get_4 _output_get_2 _output_get_3 ignoreActors)))

(fn `DrawShotDirectionArrow`
  (bind _returnvalue (not (`self.isMoving`)))
  (`self.ToggleArrow` _returnvalue)
  (if _returnvalue
    (`self.SetArrowDirection` (`self.launchDirection`))))

(fn `IncreaseLaunchPower`
  (bind _returnvalue (+ (`self.currentShotPower`) (* (`self.deltaTime`) (`self.launchPowerIncrementRate`))))
  (`self.SetLaunchPower` _returnvalue)
  (`KismetSystemLibrary.PrintString` (`KismetStringLibrary.Conv_DoubleToString` _returnvalue) true true (struct :`G` 0.66 :`B` 1.0 :`A` 1.0) 0.0))

(fn `JumpToLastLaunchPosition`
  (`KismetSystemLibrary.PrintString` "jump to last launch position")
  (`self.K2_SetActorLocation` (`self.lastLaunchPosition`))
  (`PrimitiveComponent.SetPhysicsLinearVelocity` (`self.GolfBallMesh`) (0.0 0.0 0.0) false "None")
  (`self.ResetLaunchDirection`)
  (`self.ResetLaunchPower`))

(fn `MultiplyArrowScale`
  (params (scaleFactor :type "Float (double-precision)"))
  (locals (fullScaleColor :type "LinearColor Structure" :default (struct :`R` 0.5625)) (initialScaleColor :type "LinearColor Structure" :default (struct :`R` 1.0 :`G` 0.5)))
  (bind _arrow (`self.arrow`))
  (`SceneComponent.SetRelativeScale3D` _arrow (* (`self.initialArrowScale`) (+ (* scaleFactor 0.4) 1.0)))
  (bind _returnvalue (`PrimitiveComponent.CreateDynamicMaterialInstance` _arrow 0 (`PrimitiveComponent.GetMaterial` _arrow 0) "None"))
  (`MaterialInstanceDynamic.SetVectorParameterValue` _returnvalue "emissiveColor" (`KismetMathLibrary.LinearColorLerp` (`local.initialScaleColor`) (`local.fullScaleColor`) scaleFactor)))

(fn `OnTakeShot`
  (bind _lasersightparticles (`self.laserSightParticles`))
  (set `self.isCharging` false)
  (`self.ResetLaunchPower`)
  (`self.ResetLaunchDirection`)
  ;[1 1 1] Increase number of shots taken
  (bind _returnvalue (`GameplayStatics.GetActorOfClass` "/Game/_MiniGolf/Blueprints/Managers/SceneInfo.SceneInfo_C"))
  (set `/Game/_MiniGolf/Blueprints/Managers/SceneInfo.shotsTaken` (+ (`/Game/_MiniGolf/Blueprints/Managers/SceneInfo.shotsTaken` _returnvalue) 1) _returnvalue)
  ;[1 1 1] Reset particles array
  (set `self.currentLaserRays` 0)
  (set `self.isLaserAllowed` false)
  (for _array_element _lasersightparticles
    ;;[0.3252 0.9001 1] loop body
    (`ActorComponent.K2_DestroyComponent` _array_element))
  (`KismetArrayLibrary.Array_Clear` _lasersightparticles))

(fn `ResetArrowScale`
  (locals (initialScaleColor :type "LinearColor Structure" :default (struct :`R` 1.0 :`G` 0.5)))
  (bind _arrow (`self.arrow`))
  (`SceneComponent.SetRelativeScale3D` _arrow (`self.initialArrowScale`))
  (bind _returnvalue (`PrimitiveComponent.CreateDynamicMaterialInstance` _arrow 0 (`PrimitiveComponent.GetMaterial` _arrow 0) "None"))
  (`MaterialInstanceDynamic.SetVectorParameterValue` _returnvalue "emissiveColor" (`local.initialScaleColor`)))

(fn `ResetLaunchDirection`
  (set `self.currentShotPitch` 0.0))

(fn `ResetLaunchPower`
  (set `self.currentShotPower` 0.0))

(fn `SetArrowDirection`
  (params (arrowFwd :type "Vector Structure"))
  (`self.K2_SetActorRotation` (`KismetMathLibrary.Conv_VectorToRotator` arrowFwd)))

(fn `SetBallColor`
  (params (color :type "LinearColor Structure"))
  (bind _returnvalue (`PrimitiveComponent.CreateDynamicMaterialInstance` (`self.GolfBallMesh`) 0 "/Game/_MiniGolf/Graphics/Models/MiniGolfGraphicsPack/Textures/MT_Ball.MT_Ball" "None"))
  (`MaterialInstanceDynamic.SetVectorParameterValue` _returnvalue "baseColor" color)
  (`PrimitiveComponent.SetMaterial` (`self.GolfBallMesh`) 0 _returnvalue))

(fn `SetIsMoving`
  (bind _output_get (set `self.currentVelocity` (`KismetMathLibrary.VSize` (`SceneComponent.GetComponentVelocity` (`self.GolfBallMesh`)))))
  (`KismetSystemLibrary.PrintString` (`KismetStringLibrary.Conv_DoubleToString` _output_get) true true (struct :`R` 1.0 :`G` 0.946138 :`A` 1.0) 0.0)
  (bind _output_get_2 (set `self.isMoving` (> _output_get (`self.isMovingThreshold`))))
  (if _output_get_2
    (if (not (`self.isInMagnet`))
      (`self.ApplyManualFriction`))
    (else
      (`self.StopAllMovement`)
      (`self.ResetArrowScale`))))

(fn `SetLastLaunchPosition`
  (params (pos :type "Vector Structure"))
  (set `self.lastLaunchPosition` pos))

(fn `SetLaunchDirection`
  (set `self.launchDirection` (`KismetMathLibrary.GetForwardVector` (`KismetMathLibrary.MakeRotator` 0.0 (`self.currentShotPitch`) (`self.currentShotYaw`)))))

(fn `SetLaunchPower`
  (params (power :type "Float (double-precision)"))
  (bind _asgolf_game_instance (cast `/Game/_MiniGolf/Blueprints/Managers/GolfGameInstance` (`GameplayStatics.GetGameInstance`)))
  (set `self.currentShotPower` (`KismetMathLibrary.FClamp` power 0.0 (`/Game/_MiniGolf/Blueprints/Managers/GolfGameInstance.skill_maxLaunchPower` _asgolf_game_instance))))

(fn `SetMinMaxCameraPitch`
  (params (min :type "Float (double-precision)") (max :type "Float (double-precision)"))
  (bind _returnvalue (`GameplayStatics.GetPlayerCameraManager` 0))
  (set `PlayerCameraManager.ViewPitchMin` min _returnvalue)
  (set `PlayerCameraManager.ViewPitchMax` max _returnvalue))

(fn `SetShotPitch`
  (params (mouseScrollVal :type "Float (double-precision)"))
  (returns (pitchAngle :type "Float (double-precision)"))
  (bind _returnvalue (`KismetMathLibrary.FClamp` (+ (`self.currentShotPitch`) (* mouseScrollVal (`self.anglesPerScroll`))) -45.0 80.0))
  (`KismetSystemLibrary.PrintString` (`KismetStringLibrary.Conv_DoubleToString` _returnvalue) true true (struct :`R` 0.07485 :`G` 1.0 :`B` 0.164862 :`A` 1.0) 0.0)
  (bind _output_get (set `self.currentShotPitch` _returnvalue))
  (return _output_get))

(fn `SetShotYaw`
  (set `self.currentShotYaw` (.yaw (`self.GetControlRotation`))))

(fn `SteerTowardsHole`
  (locals (maxAttractionSpeed :type "Float (double-precision)" :default 35.0) (maxSteeringForce :type "Float (double-precision)" :default 1.5) (desiredVelocity :type "Vector Structure") (steer :type "Vector Structure"))
  (bind _golfballmesh (`self.GolfBallMesh`))
  ;[1 1 1] if ball is within magnet radius
  (bind _asgolf_game_mode (cast `/Game/_MiniGolf/Blueprints/Managers/GolfGameMode` (`GameplayStatics.GetGameMode`)))
  (bind _currentsceneinfo (`/Game/_MiniGolf/Blueprints/Managers/GolfGameMode.currentSceneInfo` _asgolf_game_mode))
  (bind _ballhole (`/Game/_MiniGolf/Blueprints/Managers/SceneInfo.ballHole` _currentsceneinfo))
  ;[1 1 1] Steer towards hole
  (if (and (<= (`/Game/_MiniGolf/Blueprints/Managers/SceneInfo.distanceToHole` _currentsceneinfo) (`/Game/_MiniGolf/Blueprints/GameComponents/Hole.magnetRadius` _ballhole)) (`SceneComponent.IsSimulatingPhysics` (`self.GolfBallMesh`) "None"))
    (`KismetSystemLibrary.PrintString` "steering towards hole" true true (struct :`G` 0.66 :`B` 1.0 :`A` 1.0) 0.0)
    (set `self.isInMagnet` true)
    (bind _output_get (set `local.desiredVelocity` (* (`KismetMathLibrary.GetDirectionUnitVector` (`self.K2_GetActorLocation`) (`SceneComponent.K2_GetComponentLocation` (`/Game/_MiniGolf/Blueprints/GameComponents/Hole.magneticField` _ballhole))) (`local.maxAttractionSpeed`))))
    (bind _returnvalue (`PrimitiveComponent.GetPhysicsLinearVelocity` _golfballmesh "None"))
    (bind _output_get_2 (set `local.steer` (* (- _output_get _returnvalue) (`local.maxSteeringForce`))))
    (`PrimitiveComponent.AddForce` _golfballmesh _output_get_2 "None" false)
    (else
      (set `self.isInMagnet` false))))

(fn `StopAllMovement`
  (`PrimitiveComponent.SetPhysicsLinearVelocity` (`self.GolfBallMesh`) (0.0 0.0 0.0) false "None")
  (`self.K2_SetActorRotation` (`self.K2_GetActorRotation`))
  (`PrimitiveComponent.SetPhysicsAngularVelocityInDegrees` (`self.GolfBallMesh`) (0.0 0.0 0.0) false "None"))

(fn `TakeShot`
  (`PrimitiveComponent.SetPhysicsLinearVelocity` (`self.GolfBallMesh`) (* (`self.launchDirection`) (`self.currentShotPower`)) false "None")
  (`GameplayStatics.PlaySoundAtLocation` "/Game/_MiniGolf/Sounds/SFXs/takeShot.takeShot" (`self.K2_GetActorLocation`) (struct) 1.0 1.0 0.0 null null null))

(fn `ToggleArrow`
  (params (isActive :type Boolean))
  (`SceneComponent.SetVisibility` (`self.arrow`) isActive false))

(fn `UpdateShotPitchUI`
  (params (pitchAngle :type "Float (double-precision)"))
  (bind _asgolf_game_mode (cast `/Game/_MiniGolf/Blueprints/Managers/GolfGameMode` (`GameplayStatics.GetGameMode`)))
  (`Widget.SetRenderTransformAngle` (`/Game/_MiniGolf/Widgets/Widget_3GameplayHUD.arrow-top` (`/Game/_MiniGolf/Blueprints/Managers/SceneInfo.hudWidget` (`/Game/_MiniGolf/Blueprints/Managers/GolfGameMode.currentSceneInfo` _asgolf_game_mode))) (* -1 pitchAngle)))

(fn `UserConstructionScript`
  (set `self.initialArrowScale` (`SceneComponent.RelativeScale3D` (`self.arrow`))))