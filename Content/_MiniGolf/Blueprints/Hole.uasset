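; Mini-golf hole actor that loads the next level when the player's pawn overlaps it.
; Begin overlap calls CheckForPAR, which despite its name only checks for player pawn 0, prints its name and opens the level named by NextLevel.
; End overlap prints a debug string, but compares the leaving actor to the player controller rather than the pawn.
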(event `self.ReceiveActorBeginOverlap`
  (params (OtherActor :type "Actor Object Reference"))
  (`self.CheckForPAR` OtherActor))

(event `self.ReceiveActorEndOverlap`
  (params (OtherActor :type "Actor Object Reference"))
  (if (== OtherActor (`GameplayStatics.GetPlayerController` 0))
    (`KismetSystemLibrary.PrintString` "OnTriggerExit")))

(fn `CheckForPAR`
  (params (other :type "Actor Object Reference"))
  (if (== other (`GameplayStatics.GetPlayerPawn` 0))
    (`KismetSystemLibrary.PrintString` (`KismetSystemLibrary.GetDisplayName` other))
    (`GameplayStatics.OpenLevel` (`KismetStringLibrary.Conv_StringToName` (`self.nextLevel`)))))

(fn `UserConstructionScript`)